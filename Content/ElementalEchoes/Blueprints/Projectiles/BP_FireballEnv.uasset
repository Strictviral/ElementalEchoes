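; BP_FireballEnv is an environmental fireball projectile that kills certain player characters on contact.
; On BeginPlay it sets its ProjectileMovement velocity along local forward, then destroys itself after LifeTimeDuration.
; Sphere overlaps cast to BP_BaseCharacter and switch on CharacterName: Toast and Tremor trigger HandleDeath and destroy the fireball, while other overlaps have no scripted effect.
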(event `self.ReceiveBeginPlay`
  (`ProjectileMovementComponent.SetVelocityInLocalSpace` (`self.ProjectileMovement`) (500.0 0.0 0.0))
  (`KismetSystemLibrary.Delay` (`self.LifeTimeDuration`))
  (`self.K2_DestroyActor`))

(event `self.Sphere.OnComponentBeginOverlap`
  (params (OverlappedComponent :type "PrimitiveComponent Object Reference") (OtherActor :type "Actor Object Reference") (OtherComp :type "PrimitiveComponent Object Reference") (OtherBodyIndex :type Integer) (bFromSweep :type Boolean) (SweepResult :type "HitResult Structure (by ref)"))
  (bind _asbp_base_character (cast `/Game/ElementalEchoes/Blueprints/Character/BP_BaseCharacter` OtherActor))
  (switch `string` (`/Game/ElementalEchoes/Blueprints/Character/BP_BaseCharacter.CharacterName` _asbp_base_character)
    (:`Toast`
      (`/Game/ElementalEchoes/Blueprints/Character/BP_BaseCharacter.HandleDeath` _asbp_base_character)
      (`self.K2_DestroyActor`))
    (:`Tremor`
      (`/Game/ElementalEchoes/Blueprints/Character/BP_BaseCharacter.HandleDeath` _asbp_base_character)
      (`self.K2_DestroyActor`))))

(fn `UserConstructionScript`)