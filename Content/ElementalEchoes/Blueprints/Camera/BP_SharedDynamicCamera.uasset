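; Shared camera actor that frames the fire and earth characters together, repositioning every tick after a short startup delay.
; It sits at the players' X/Z midpoint plus a height offset, deriving Y depth from their clamped separation and Player1's Y.
; Left and right line traces from the midpoint detect walls, feeding a small distance-mapped offset into the position.
; A spring-arm zoom function exists but never runs.
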(event `self.ReceiveBeginPlay`
  (`KismetSystemLibrary.Delay` 0.2)
  (`self.GetPlayers`)
  (set `self.bCanBegin` true))

(event `self.ReceiveTick`
  (params (DeltaSeconds :type "Float (single-precision)"))
  (if (`self.bCanBegin`)
    (`self.SetCameraLocation`)))

(fn `GetDistanceBetweenPlayers`
  (returns (DistanceBetweenPlayers :type "Float (double-precision)"))
  (bind (_returnvalue_x _returnvalue_y) (`KismetMathLibrary.BreakVector` (`self.K2_GetActorLocation` (`self.Player1`))))
  (return (+ (/ (`KismetMathLibrary.FClamp` (`self.GetDistanceTo` (`self.Player1`) (`self.Player2`)) (`self.Minimum Camera Zoom`) (`self.Maximum Camera Zoom`)) 2.0) _returnvalue_y)))

(fn `GetMidPointBetweenPlayers`
  (returns (MidpointDistanceBetweenPlayers :type "Vector Structure") (`World Location of Player` :type "Vector Structure"))
  (bind (_wall_detetct_out_hit_bblockinghit _wall_detetct_out_hit_binitialoverlap _wall_detetct_out_hit_time _wall_detetct_out_hit_distance) (`GameplayStatics.BreakHitResult` (`self.Wall Detetct Out Hit`)))
  (bind (_returnvalue_x _returnvalue_y _returnvalue_z) (`KismetMathLibrary.BreakVector` (/ (+ (`self.K2_GetActorLocation` (`self.Player1`)) (`self.K2_GetActorLocation` (`self.Player2`))) 2.0)))
  (bind _distancebetweenplayers (`self.GetDistanceBetweenPlayers`))
  (set `self.MidPoint` (`KismetMathLibrary.MakeVector` _returnvalue_x _distancebetweenplayers _returnvalue_z))
  (return (+ (`self.MidPoint`) (`KismetMathLibrary.SelectFloat` (`KismetMathLibrary.MapRangeClamped` _wall_detetct_out_hit_distance (`self.WallDetectionRadius`) 0.0 1.0 -1.0) 1.0 (or (`self.WallDetectedLeft`) (`self.WallDetectedRight`)))) (`KismetMathLibrary.MakeVector` _returnvalue_x _returnvalue_y _returnvalue_z)))

(fn `GetPlayers`
  (bind _returnvalue (`GameplayStatics.GetActorOfClass` "/Game/ElementalEchoes/Blueprints/Character/BP_FireCharacter.BP_FireCharacter_C"))
  (set `self.Player1` _returnvalue)
  (bind _returnvalue_2 (`GameplayStatics.GetActorOfClass` "/Game/ElementalEchoes/Blueprints/Character/BP_EarthCharacter.BP_EarthCharacter_C"))
  (set `self.Player2` _returnvalue_2))

(fn `SetCameraLocation`
  (bind (_midpointdistancebetweenplayers _world_location_of_player) (`self.GetMidPointBetweenPlayers`))
  (`self.WallCheckTrace` _world_location_of_player)
  (`self.K2_SetActorLocation` (`KismetMathLibrary.MakeVector` (.x _midpointdistancebetweenplayers) (.y _midpointdistancebetweenplayers) (+ (.z _midpointdistancebetweenplayers) (`self.CameraHeight`)))))

(fn `SetCameraSpringArmZoom`
  (bind _distancebetweenplayers (`self.GetDistanceBetweenPlayers`))
  (set `SpringArmComponent.TargetArmLength` (`KismetMathLibrary.FClamp` _distancebetweenplayers 0.0 650.0) (`self.SpringArm`)))

(fn `UserConstructionScript`)

(fn `WallCheckTrace`
  (params (MidPointPlayerLocation :type "Vector Structure"))
  (bind (_outhit _returnvalue) (`KismetSystemLibrary.LineTraceSingle` :`Start` MidPointPlayerLocation :`End` (+ MidPointPlayerLocation (* (`KismetMathLibrary.NegateVector` (`self.GetActorRightVector`)) (`self.WallDetectionRadius`))) :`TraceChannel` "TraceTypeQuery3" :`DrawDebugType` "ForOneFrame" :`TraceColor` (struct :`R` 0.015005 :`G` 0.018871 :`B` 1.0 :`A` 1.0) :`TraceHitColor` (struct :`R` 1.0 :`G` 0.000929 :`A` 1.0)))
  (if _returnvalue
    (set `self.WallDetectedLeft` true)
    (set `self.Wall Detetct Out Hit` _outhit)
    (else
      (set `self.WallDetectedLeft` false)))
  (bind (_outhit_2 _returnvalue_2) (`KismetSystemLibrary.LineTraceSingle` :`Start` MidPointPlayerLocation :`End` (+ MidPointPlayerLocation (* (`self.GetActorRightVector`) (`self.WallDetectionRadius`))) :`TraceChannel` "TraceTypeQuery4" :`DrawDebugType` "ForOneFrame" :`TraceColor` (struct :`R` 0.915517 :`G` 1.0 :`A` 1.0)))
  (if _returnvalue_2
    (set `self.WallDetectedRight` true)
    (set `self.Wall Detetct Out Hit` _outhit_2)
    (else
      (set `self.WallDetectedRight` false)
      (if (not (or (`self.WallDetectedRight`) (`self.WallDetectedLeft`)))
        (set `self.Wall Detetct Out Hit` (struct))))))