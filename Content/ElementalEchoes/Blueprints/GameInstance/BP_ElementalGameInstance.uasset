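; Game instance for Elemental Echoes that persists audio settings and tracks the player's most recent checkpoint location.
; On Init it loads or creates a BP_SaveSettings object and seeds the checkpoint from the level's PlayerStart.
; Master, music and SFX volume events write into that object and immediately save it to its slot.
; Checkpoint functions set, get or zero the location, which is held only in memory.
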(event `self.ReceiveInit`
  ; Init
  (`self.LoadSettings`)
  (`self.InitializeCheckpointLocation`))

(event `LoadSettings`
  ; Load Save Slot
  (bind _returnvalue (`GameplayStatics.DoesSaveGameExist` (`self.SettingsSlot`)))
  (if _returnvalue
    (bind _returnvalue_2 (`GameplayStatics.LoadGameFromSlot` (`self.SettingsSlot`)))
    (bind _asbp_save_settings (cast `/Game/ElementalEchoes/Blueprints/SaveGame/BP_SaveSettings` _returnvalue_2))
    (set `self.BP_SaveSettings` _asbp_save_settings)
    (else
      (bind _returnvalue_3 (`GameplayStatics.CreateSaveGameObject` "/Game/ElementalEchoes/Blueprints/SaveGame/BP_SaveSettings.BP_SaveSettings_C"))
      (set `self.BP_SaveSettings` _returnvalue_3))))

(event `Save Settings`
  ; Save game to slot
  (bind _returnvalue (`GameplayStatics.SaveGameToSlot` (`self.BP_SaveSettings`) (`self.SettingsSlot`)))
  (if _returnvalue
    (`KismetSystemLibrary.PrintString` "Saved")))

(event `Save Volume SFX`
  (params (`SFX Volume` :type "Float (double-precision)"))
  ; Save each volume value
  (set `/Game/ElementalEchoes/Blueprints/SaveGame/BP_SaveSettings.SFXVolume` `SFX Volume` (`self.BP_SaveSettings`))
  (`self.Save Settings`))

(event `Save Volume Music`
  (params (`Music Volume` :type "Float (double-precision)"))
  ; Save each volume value
  (set `/Game/ElementalEchoes/Blueprints/SaveGame/BP_SaveSettings.MusicVolume` `Music Volume` (`self.BP_SaveSettings`))
  (`self.Save Settings`))

(event `Save Volume Master`
  (params (`Master Volume` :type "Float (double-precision)"))
  ; Save each volume value
  (set `/Game/ElementalEchoes/Blueprints/SaveGame/BP_SaveSettings.MasterVolume` `Master Volume` (`self.BP_SaveSettings`))
  (`self.Save Settings`))

(fn `ClearCheckpoints`
  (set `self.MostRecentCheckpointLocation` (0.0 0.0 0.0)))

(fn `GetRecentCheckpoint`
  (returns (RecentCheckpoint :type "Vector Structure"))
  (return (`self.MostRecentCheckpointLocation`)))

(fn `InitializeCheckpointLocation`
  (bind _returnvalue (`GameplayStatics.GetActorOfClass` "/Script/Engine.PlayerStart"))
  (set `self.MostRecentCheckpointLocation` (`Actor.K2_GetActorLocation` _returnvalue)))

(fn `SetRecentCheckpoint`
  (params (NewCheckpointLocation :type "Vector Structure"))
  (set `self.MostRecentCheckpointLocation` NewCheckpointLocation))