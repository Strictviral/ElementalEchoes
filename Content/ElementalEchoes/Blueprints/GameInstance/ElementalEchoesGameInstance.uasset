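; Game instance for Elemental Echoes that tries to gather player controllers into an array on Init.
; GetPlayersControllers checks validity once at the current index, then runs a fixed loop that stores each controller and increments the index.
; Each pass prints the controller at the incremented index, one past the stored one, and a failed check prints a debug message.
; An unconnected, empty loop is also left in the graph.
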(event `self.ReceiveInit`
  (`self.GetPlayersControllers`))

(fn `GetPlayersControllers`
  (bind _returnvalue (`GameplayStatics.GetPlayerController` (`self.Loop integer`)))
  (`/Engine/EditorBlueprintResources/StandardMacros.IsValid` _returnvalue
    (:`Is Valid`
      (for _ (range 4)
        (`KismetArrayLibrary.Array_Add` (`self.ArrayOfControllers`) _returnvalue)
        (`/Engine/EditorBlueprintResources/StandardMacros.IncrementInt` (`self.Loop integer`)
          (:`  `
            (`KismetSystemLibrary.PrintString` (`KismetSystemLibrary.GetDisplayName` _returnvalue))))))
    (:`Is Not Valid`
      (`KismetSystemLibrary.PrintString` "No more controlelrs"))))