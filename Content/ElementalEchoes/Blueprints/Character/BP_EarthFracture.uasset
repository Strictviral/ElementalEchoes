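; BP_EarthFracture is a short-lived debris actor that scatters the separate body-part meshes of what appears to be an earth character.
; The construction script gathers the face, middle face, fingers, legs and arm meshes into an array.
; On BeginPlay, each valid mesh receives a random impulse along X and Z only, then the actor destroys itself after a brief delay.
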(event `self.ReceiveBeginPlay`
  (for _array_element (`self.MeshComponents`)
    (`/Engine/EditorBlueprintResources/StandardMacros.IsValid` _array_element
      (:`Is Valid`
        (`PrimitiveComponent.AddImpulse` _array_element (`KismetMathLibrary.MakeVector` (`KismetMathLibrary.RandomFloatInRange` -10000.0 10000.0) 0.0 (`KismetMathLibrary.RandomFloatInRange` -10000.0 10000.0)) "None" false))))
  (`KismetSystemLibrary.Delay` 2.0)
  (`self.K2_DestroyActor`))

(fn `UserConstructionScript`
  (`KismetArrayLibrary.Array_AddUnique` (`self.MeshComponents`) (`self.FaceMesh`))
  (`KismetArrayLibrary.Array_AddUnique` (`self.MeshComponents`) (`self.MiddleFaceMesh`))
  (`KismetArrayLibrary.Array_AddUnique` (`self.MeshComponents`) (`self.Fingers`))
  (`KismetArrayLibrary.Array_AddUnique` (`self.MeshComponents`) (`self.Legs`))
  (`KismetArrayLibrary.Array_AddUnique` (`self.MeshComponents`) (`self.ArmMesh`)))