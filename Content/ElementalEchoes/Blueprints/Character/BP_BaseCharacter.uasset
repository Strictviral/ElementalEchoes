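; Base player character for Elemental Echoes, handling death, checkpoint respawn, pausing, interaction and left/right facing.
; Death shows an indicator above the capsule, disables input, collision and movement, then respawns after a delay at the GameInstance's latest checkpoint unless the game has ended.
; Pausing opens WBP_Pause, whose events resume or reload the checkpoint, and swaps Enhanced Input mapping contexts on every PlayerController.
; Helpers trigger the first overlapping BPI_Interact actor and flip rotation by move input.
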(event `self.ReceivePossessed`
  (params (NewController :type "Controller Object Reference"))
  (bind _asbp_elemental_controller (cast `/Game/ElementalEchoes/Blueprints/Controller/BP_ElementalController` NewController))
  (set `self.PlayerOwnedController` _asbp_elemental_controller))

(event `self.ReceiveBeginPlay`
  (`parent.ReceiveBeginPlay`)
  (`KismetSystemLibrary.Delay` 0.2)
  (bind _asbp_elemental_controller (cast `/Game/ElementalEchoes/Blueprints/Controller/BP_ElementalController` (`self.GetLocalViewingPlayerController`))
    (:`then`
      (set `self.PlayerOwnedController` _asbp_elemental_controller))
    (:`CastFailed`
      _))
  (bind _asbp_elemental_game_instance (cast `/Game/ElementalEchoes/Blueprints/GameInstance/BP_ElementalGameInstance` (`GameplayStatics.GetGameInstance`)))
  (set `self.ElementalGameInstance` _asbp_elemental_game_instance))

(event `HandleDeath`
  (bind _deathindicator_widget (`self.DeathIndicator_Widget`))
  (bind _playerownedcontroller (`self.PlayerOwnedController`))
  ; Handles Spawning of Character
  (`self.AddDeadPlayers`)
  (`/Engine/EditorBlueprintResources/StandardMacros.IsValid` _playerownedcontroller
    (:`Is Valid`
      (bind _returnvalue (`|CreateWidget` "/Game/ElementalEchoes/Blueprints/UI/WBP_DeathIndicator.WBP_DeathIndicator_C" _playerownedcontroller))
      (bind _output_get (set `self.DeathIndicator Widget` _returnvalue))
      (`WidgetComponent.SetWidget` _deathindicator_widget _output_get)
      (`WidgetComponent.SetDrawSize` _deathindicator_widget (130.0 110.0))
      (`SceneComponent.K2_SetRelativeLocation` _deathindicator_widget (`KismetMathLibrary.MakeVector` 0.0 0.0 (+ (`CapsuleComponent.CapsuleHalfHeight` (`self.CapsuleComponent`)) 50.0)) false false)
      (`SceneComponent.SetVisibility` _deathindicator_widget true false)
      (`self.DisableInput` (`self.PlayerOwnedController`))
      (`PrimitiveComponent.SetCollisionEnabled` (`self.CapsuleComponent`) "NoCollision")
      (`ActorComponent.SetActive` (`self.CharacterMovement`) false false)
      (`KismetSystemLibrary.Delay` 2.0)
      (if (not (`self.bHasGameEnded`))
        (`self.Respawn`)))))

(event `Reload Checkpoint (From Menu)`
  ; Handles Spawning of Character
  ;; Respawn Event
  (`self.RemoveDeadPlayers` :!label _label)
  (`KismetSystemLibrary.PrintString` "Respawn")
  (`self.K2_SetActorLocation` (`/Game/ElementalEchoes/Blueprints/GameInstance/BP_ElementalGameInstance.MostRecentCheckpointLocation` (`self.ElementalGameInstance`)))
  (`SceneComponent.SetVisibility` (`self.DeathIndicator_Widget`) false false)
  (`Widget.RemoveFromParent` (`self.DeathIndicator Widget`))
  (`self.EnableInput` (`self.PlayerOwnedController`))
  (`PrimitiveComponent.SetCollisionEnabled` (`self.CapsuleComponent`) "QueryAndPhysics")
  (`ActorComponent.SetActive` (`self.CharacterMovement`) true false))

(event `Respawn`
  ; Handles Spawning of Character
  ;; Respawn Event
  (goto _label))

(event `EnhancedInput|/Game/ElementalEchoes/Blueprints/Controller/InputActions/UI_Input/IA_Pause`
  (params (ActionValue :type Boolean) (ElapsedSeconds :type "Float (double-precision)") (TriggeredSeconds :type "Float (double-precision)") (InputAction :type "InputAction Object Reference" :default "/Game/ElementalEchoes/Blueprints/Controller/InputActions/UI_Input/IA_Pause.IA_Pause"))
  (bind _pause_widget (`self.Pause Widget`))
  ; Pause
  (:`Started`
    (if (not (`self.bIsPaused`))
      (bind _returnvalue (`|CreateWidget` "/Game/ElementalEchoes/Blueprints/UI/WBP_Pause.WBP_Pause_C"))
      (bind _output_get (set `self.Pause Widget` _returnvalue))
      (add `/Game/ElementalEchoes/Blueprints/UI/WBP_Pause.E_Reload Checkpoint` _output_get (delegate `Reload Checkpoint From UI`))
      (add `/Game/ElementalEchoes/Blueprints/UI/WBP_Pause.E_Resume Game` _output_get (delegate `Resume Game`))
      (`self.ChangeMappingContext to UI`)
      (set `self.bIsPaused` true)
      (`KismetSystemLibrary.PrintString` "Pause Game")
      (`GameplayStatics.SetGamePaused` true)
      (`/Game/ElementalEchoes/Blueprints/UI/WBP_Pause.Initialise` _pause_widget (`self.PlayerOwnedController`))
      (`UserWidget.AddToViewport` _pause_widget 0)
      (`Widget.SetFocus` (`/Game/ElementalEchoes/Blueprints/UI/WBP_Pause.WBP_Button_Resume` _pause_widget)))))

(event `Resume Game`
  ; Pause
  (`self.ResumeGame`))

(event `Reload Checkpoint From UI`
  ; Pause
  (if (`self.bHasACheckpoint`)
    (`self.K2_SetActorLocation` (`/Game/ElementalEchoes/Blueprints/GameInstance/BP_ElementalGameInstance.MostRecentCheckpointLocation` (`self.ElementalGameInstance`)))
    (`self.ChangeMappingContext to Gameplay`)
    (set `self.bIsPaused` false)
    (`GameplayStatics.SetGamePaused` false)
    (`Widget.RemoveFromParent` (`self.Pause Widget`))
    (else
      (`KismetSystemLibrary.PrintString` "No Checkpoint"))))

(fn `ChangeMappingContext to Gameplay`
  (bind _outactors (`GameplayStatics.GetAllActorsOfClass` "/Script/Engine.PlayerController"))
  (for _array_element _outactors
    (bind _returnvalue (pcsubsystem `EnhancedInputLocalPlayerSubsystem` _array_element))
    (`EnhancedInputSubsystemInterface.AddMappingContext` _returnvalue "/Game/ElementalEchoes/Blueprints/Controller/IMC_ElementalMappingContext.IMC_ElementalMappingContext" 0 (struct))
    (`KismetSystemLibrary.PrintString` "Mapping to Game" true true (struct :`R` 1.0 :`B` 0.361135 :`A` 1.0))
    (`EnhancedInputSubsystemInterface.RemoveMappingContext` _returnvalue "/Game/ElementalEchoes/Blueprints/Controller/IMC_ElementalUI.IMC_ElementalUI" (struct))))

(fn `ChangeMappingContext to UI`
  (bind _outactors (`GameplayStatics.GetAllActorsOfClass` "/Script/Engine.PlayerController"))
  (for _array_element _outactors
    (bind _returnvalue (pcsubsystem `EnhancedInputLocalPlayerSubsystem` _array_element))
    (`EnhancedInputSubsystemInterface.AddMappingContext` _returnvalue "/Game/ElementalEchoes/Blueprints/Controller/IMC_ElementalUI.IMC_ElementalUI" 1 (struct))
    (`KismetSystemLibrary.PrintString` "Mapping to UI")
    (`EnhancedInputSubsystemInterface.RemoveMappingContext` _returnvalue "/Game/ElementalEchoes/Blueprints/Controller/IMC_ElementalMappingContext.IMC_ElementalMappingContext" (struct))
    (`KismetSystemLibrary.PrintString` (`KismetSystemLibrary.GetDisplayName` _array_element))))

(fn `CheckForInteractableObjects`
  (for _array_element (`self.GetOverlappingActors` "/Script/Engine.Actor")
    (if (`KismetSystemLibrary.DoesImplementInterface` _array_element "/Game/ElementalEchoes/Blueprints/Interface/BPI_Interact.BPI_Interact_C")
      (message `/Game/ElementalEchoes/Blueprints/Interface/BPI_Interact.Interact` _array_element)
      (break))))

(fn `ResumeGame`
  (`Widget.RemoveFromParent` (`self.Pause Widget`))
  (`KismetSystemLibrary.PrintString` "UnPause Game")
  (`GameplayStatics.SetGamePaused` false)
  (`self.ChangeMappingContext to Gameplay`)
  (set `self.bIsPaused` false))

(fn `RotateCharacter`
  (params (MoveInputValue :type "Float (double-precision)"))
  (if (> MoveInputValue 0.1)
    (`self.K2_SetActorRotation` (struct))
    (elif (< MoveInputValue -0.1)
      (`self.K2_SetActorRotation` (struct :`Yaw` 180.0)))))

(fn `UserConstructionScript`
  (`parent.UserConstructionScript`))