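; Earth-element player character with stone pillar, shield brace and push/pull abilities, built on a parent character class.
; Enhanced Input previews and triggers pillars, and toggles a brace that locks movement and spawns a rotatable shield, removed on death.
; Push/pull functions box-trace for movable objects or spheres, disable their physics and attach them to an anchor.
; State flags and movement settings restrict conflicting actions while pushing or braced.
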(event `self.ReceiveBeginPlay`
  (`parent.ReceiveBeginPlay`)
  (bind _returnvalue (`|SpawnActorFromClass` "/Game/ElementalEchoes/Blueprints/Character/CharacterAbilities/EarthAbilities/BP_EarthShield.BP_EarthShield_C" (`KismetMathLibrary.MakeTransform` (0.0 0.0 0.0)) "Undefined" "MultiplyWithRoot" null null))
  (`self.K2_AttachToComponent` _returnvalue (`self.Mesh`) "ShieldSocket" "SnapToTarget" "SnapToTarget" "KeepRelative" true))

(event `EnhancedInput|/Game/ElementalEchoes/Blueprints/Controller/InputActions/IA_AbilityRT_Earth`
  (params (ActionValue :type Boolean) (ElapsedSeconds :type "Float (double-precision)") (TriggeredSeconds :type "Float (double-precision)") (InputAction :type "InputAction Object Reference" :default "/Game/ElementalEchoes/Blueprints/Controller/InputActions/IA_AbilityRT_Earth.IA_AbilityRT_Earth"))
  ; Controls Spawning the Pillar
  (:`Triggered`
    (`self.SpawnStonePillar`))
  (:`Started`
    (bind _returnvalue (`self.SpawnIndicator`)))
  (:`Canceled`
    (`self.K2_DestroyActor` _returnvalue)
    (set `self.bCanSpawnPillar` true)))

(event `EnhancedInput|/Game/ElementalEchoes/Blueprints/Controller/InputActions/IA_RotateShield`
  (params (ActionValue :type "Vector2D Structure") (ElapsedSeconds :type "Float (double-precision)") (TriggeredSeconds :type "Float (double-precision)") (InputAction :type "InputAction Object Reference" :default "/Game/ElementalEchoes/Blueprints/Controller/InputActions/IA_RotateShield.IA_RotateShield"))
  (:`Triggered`
    (`self.CheckandRotateShield` ActionValue_Y)))

(event `EnhancedInput|/Game/ElementalEchoes/Blueprints/Controller/InputActions/IA_BaseAbility`
  (params (ActionValue :type Boolean) (ElapsedSeconds :type "Float (double-precision)") (TriggeredSeconds :type "Float (double-precision)") (InputAction :type "InputAction Object Reference" :default "/Game/ElementalEchoes/Blueprints/Controller/InputActions/IA_BaseAbility.IA_BaseAbility"))
  ; Interact Interface (Push pull)
  (:`Started`
    (`self.CheckForInteractableObjects`)))

(event `EnhancedInput|/Game/ElementalEchoes/Blueprints/Controller/InputActions/IA_Brace`
  (params (ActionValue :type Boolean) (ElapsedSeconds :type "Float (double-precision)") (TriggeredSeconds :type "Float (double-precision)") (InputAction :type "InputAction Object Reference" :default "/Game/ElementalEchoes/Blueprints/Controller/InputActions/IA_Brace.IA_Brace"))
  ; Brace Ability
  (:`Triggered`
    (if (not (`self.bIsBraced`))
      (`self.Brace`)
      (else
        (`self.StopBrace`)))))

(event `EnhancedInput|/Game/Input/Actions/IA_Move`
  (params (ActionValue :type "Vector2D Structure") (ElapsedSeconds :type "Float (double-precision)") (TriggeredSeconds :type "Float (double-precision)") (InputAction :type "InputAction Object Reference" :default "/Game/Input/Actions/IA_Move.IA_Move"))
  (:`Triggered`
    (set `self.MoveValue` ActionValue_Y)
    (if (not (`self.bIsPushing`))
      (`self.RotateCharacter` ActionValue_Y))))

(event `EnhancedInput|/Game/Input/Actions/IA_Jump`
  (params (ActionValue :type Boolean) (ElapsedSeconds :type "Float (double-precision)") (TriggeredSeconds :type "Float (double-precision)") (InputAction :type "InputAction Object Reference" :default "/Game/Input/Actions/IA_Jump.IA_Jump"))
  (:`Triggered`
    (if (and (not (`NavMovementInterface.IsFalling` (`self.CharacterMovement`))) (`self.bCanJump`))
      (`self.Jump`)
      (set `self.bCanJump` false))))

(event `self.OnLanded`
  (params (Hit :type "HitResult Structure (by ref)"))
  (set `self.bCanJump` true))

(fn `Brace`
  (bind _charactermovement (`self.CharacterMovement`))
  (bind (_returnvalue_x _returnvalue_y _returnvalue_z) (`KismetMathLibrary.BreakVector` (+ (* (`self.GetActorForwardVector`) 60.0) (`self.K2_GetActorLocation`))))
  (if (and (not (`NavMovementComponent.IsFalling` (`self.CharacterMovement`))) (`self.bcanUsedShield`))
    (set `self.bCanRotate` false)
    (set `CharacterMovementComponent.bOrientRotationToMovement` false (`self.CharacterMovement`))
    (set `CharacterMovementComponent.bUseControllerDesiredRotation` false (`self.CharacterMovement`))
    (set `self.bCanSpawnPillar` false)
    (set `self.bCanJump` false)
    (set `self.bIsBraced` true)
    (set `self.bCanPush/Pull` false)
    (set `CharacterMovementComponent.MaxWalkSpeed` 0.0 _charactermovement)
    (`CharacterMovementComponent.SetMovementMode` _charactermovement "MOVE_None" 0)
    (bind _returnvalue (`|SpawnActorFromClass` "/Game/ElementalEchoes/Blueprints/Character/CharacterAbilities/EarthAbilities/BP_EarthShieldTestReplace.BP_EarthShieldTestReplace_C" (`KismetMathLibrary.MakeTransform` (`KismetMathLibrary.MakeVector` _returnvalue_x _returnvalue_y (+ _returnvalue_z 50.0)) (struct :`Yaw` 90.0)) "Undefined" "MultiplyWithRoot" null null))
    (set `self.StoneShield` _returnvalue)))

(fn `CheckandAttachMovingObject`
  (if (`self.bCanPush/Pull`)
    (bind (_outhit _returnvalue) (`KismetSystemLibrary.BoxTraceSingle` :`Start` (`self.K2_GetActorLocation`) :`End` (+ (`self.K2_GetActorLocation`) (* (`self.GetActorForwardVector`) 100.0)) :`HalfSize` (50.0 0.0 0.0) :`TraceChannel` "TraceTypeQuery1" :`DrawDebugType` "ForDuration"))
    (if _returnvalue
      (bind _asbp_movable_objects (cast `/Game/ElementalEchoes/Blueprints/LevelActors/BP_MovableObjects` (`.HitActor` (`GameplayStatics.BreakHitResult` _outhit))))
      (set `self.bIsPushing` true)
      (`self.SetPullingVariablesForCharacter`)
      (set `self.CurrentMoveableObject` _asbp_movable_objects)
      (`PrimitiveComponent.SetSimulatePhysics` (`/Game/ElementalEchoes/Blueprints/LevelActors/BP_MovableObjects.StoneMesh` (`self.CurrentMoveableObject`)) false)
      (bind _returnvalue_2 (`self.K2_AttachToComponent` (`self.CurrentMoveableObject`) (`self.Push/PullAnchor`) "None" "KeepWorld" "KeepWorld" "KeepWorld" true))
      (if _returnvalue_2
        (`PrimitiveComponent.IgnoreActorWhenMoving` (`/Game/ElementalEchoes/Blueprints/LevelActors/BP_MovableObjects.StoneMesh` (`self.CurrentMoveableObject`)) (`Controller.K2_GetPawn` (`self.GetInstigatorController`)) true)))))

(fn `CheckandAttachMovingObjectSphere`
  (bind (_outhit _returnvalue) (`KismetSystemLibrary.BoxTraceSingle` :`Start` (`self.K2_GetActorLocation`) :`End` (+ (`self.K2_GetActorLocation`) (* (`self.GetActorForwardVector`) 100.0)) :`HalfSize` (50.0 10.0 20.0) :`TraceChannel` "TraceTypeQuery1" :`DrawDebugType` "ForDuration"))
  (if _returnvalue
    (bind _asbp_movable_sphere (cast `/Game/ElementalEchoes/Blueprints/LevelActors/BP_MovableSphere` (`.HitActor` (`GameplayStatics.BreakHitResult` _outhit))))
    (set `/Game/ElementalEchoes/Blueprints/LevelActors/BP_MovableSphere.bIsBeingPushed` true _asbp_movable_sphere)
    (set `self.CurrentSphere` _asbp_movable_sphere)
    (`self.SetPullingVariablesForCharacter`)
    (`PrimitiveComponent.SetSimulatePhysics` (`/Game/ElementalEchoes/Blueprints/LevelActors/BP_MovableSphere.StoneMesh` (`self.CurrentSphere`)) false)
    (`PrimitiveComponent.SetCollisionEnabled` (`/Game/ElementalEchoes/Blueprints/LevelActors/BP_MovableSphere.StoneMesh` (`self.CurrentSphere`)) "QueryAndPhysics")
    (bind _returnvalue_2 (`self.K2_AttachToComponent` (`self.CurrentSphere`) (`self.Push/PullAnchor`) "None" "KeepWorld" "KeepWorld" "KeepWorld" true))
    (if _returnvalue_2
      (`PrimitiveComponent.IgnoreActorWhenMoving` (`/Game/ElementalEchoes/Blueprints/LevelActors/BP_MovableSphere.StoneMesh` (`self.CurrentSphere`)) (`Controller.K2_GetPawn` (`self.GetInstigatorController`)) true))))

(fn `CheckandRotateShield`
  (params (`Y Axis` :type "Float (double-precision)"))
  (bind (_returnvalue_roll _returnvalue_pitch _returnvalue_yaw) (`KismetMathLibrary.BreakRotator` (`SceneComponent.K2_GetComponentRotation` (`/Game/ElementalEchoes/Blueprints/Character/CharacterAbilities/EarthAbilities/BP_EarthShieldTestReplace.Box` (`self.StoneShield`)))))
  (if (`self.bIsBraced`)
    (`SceneComponent.K2_SetWorldRotation` (`/Game/ElementalEchoes/Blueprints/Character/CharacterAbilities/EarthAbilities/BP_EarthShieldTestReplace.Box` (`self.StoneShield`)) (`KismetMathLibrary.MakeRotator` (+ _returnvalue_roll `Y Axis`) _returnvalue_pitch _returnvalue_yaw) false false)))

(fn `DetachFromMovingObject`
  (bind _stonemesh (`/Game/ElementalEchoes/Blueprints/LevelActors/BP_MovableObjects.StoneMesh` (`self.CurrentMoveableObject`)))
  (bind _stonemesh_2 (`/Game/ElementalEchoes/Blueprints/LevelActors/BP_MovableObjects.StoneMesh` (`self.CurrentMoveableObject`)))
  (bind _stonemesh_3 (`/Game/ElementalEchoes/Blueprints/LevelActors/BP_MovableObjects.StoneMesh` (`self.CurrentMoveableObject`)))
  (bind _returnvalue (`SceneComponent.K2_GetComponentToWorld` _stonemesh))
  (`/Engine/EditorBlueprintResources/StandardMacros.IsValid` (`self.CurrentMoveableObject`)
    (:`Is Valid`
      (set `self.bIsPushing` false)
      (`self.SetDefaultVariableForCharacter`)
      (`self.K2_DetachFromActor` (`self.CurrentMoveableObject`) "KeepWorld" "KeepWorld" "KeepWorld")
      (`KismetSystemLibrary.PrintString` (`KismetStringLibrary.Conv_TransformToString` _returnvalue))
      (`SceneComponent.K2_SetWorldTransform` _stonemesh _returnvalue false true)
      (`PrimitiveComponent.SetPhysicsLinearVelocity` _stonemesh_2 (0.0 0.0 0.0) false "None")
      (`PrimitiveComponent.SetPhysicsAngularVelocityInDegrees` _stonemesh_2 (0.0 0.0 0.0) false "None")
      (`PrimitiveComponent.SetSimulatePhysics` (`/Game/ElementalEchoes/Blueprints/LevelActors/BP_MovableObjects.StoneMesh` (`self.CurrentMoveableObject`)) true)
      (`SceneComponent.K2_SetWorldTransform` _stonemesh_3 (`SceneComponent.K2_GetComponentToWorld` _stonemesh_3) false true)
      (`PrimitiveComponent.IgnoreActorWhenMoving` (`/Game/ElementalEchoes/Blueprints/LevelActors/BP_MovableObjects.StoneMesh` (`self.CurrentMoveableObject`)) (`Controller.K2_GetPawn` (`self.GetInstigatorController`)) false))))

(fn `DetachFromMovingObjectSphere`
  (`/Engine/EditorBlueprintResources/StandardMacros.IsValid` (`self.CurrentSphere`)
    (:`Is Valid`
      (`self.SetDefaultVariableForCharacter`)
      (`self.K2_DetachFromActor` (`self.CurrentSphere`) "KeepWorld" "KeepWorld" "KeepWorld")
      (`PrimitiveComponent.SetSimulatePhysics` (`/Game/ElementalEchoes/Blueprints/LevelActors/BP_MovableSphere.StoneMesh` (`self.CurrentSphere`)) true)
      (`PrimitiveComponent.IgnoreActorWhenMoving` (`/Game/ElementalEchoes/Blueprints/LevelActors/BP_MovableSphere.StoneMesh` (`self.CurrentSphere`)) (`Controller.K2_GetPawn` (`self.GetInstigatorController`)) false))))

(fn `DisableShieldVisibility`)

(fn `EnableShieldVisibility`)

(fn `HandleDeathFunction`
  (`parent.HandleDeathFunction`)
  (`self.StopBrace`))

(fn `SetDefaultVariableForCharacter`
  (set `CharacterMovementComponent.MaxWalkSpeed` (`self.DefaultWalkSpeed`) (`self.CharacterMovement`))
  (set `CharacterMovementComponent.bOrientRotationToMovement` true (`self.CharacterMovement`))
  (set `CharacterMovementComponent.bUseControllerDesiredRotation` true (`self.CharacterMovement`))
  (set `self.bIsInteracting` false)
  (set `self.bCanJump` true)
  (set `self.bcanUsedShield` true)
  (set `self.bCanPush/Pull` true))

(fn `SetPullingVariablesForCharacter`
  (set `CharacterMovementComponent.MaxWalkSpeed` (`self.Pushing/PullingSpeed`) (`self.CharacterMovement`))
  (set `CharacterMovementComponent.bOrientRotationToMovement` false (`self.CharacterMovement`))
  (set `CharacterMovementComponent.bUseControllerDesiredRotation` false (`self.CharacterMovement`))
  (set `self.bIsInteracting` true)
  (set `self.bCanJump` false)
  (set `self.bCanSpawnPillar` false)
  (set `self.bcanUsedShield` false)
  (set `self.bCanPush/Pull` false))

(fn `SpawnIndicator`
  (returns (ReturnValue :type "/Game/ElementalEchoes/Blueprints/Character/CharacterAbilities/EarthAbilities/BP_StonePillarIndicator Object Reference"))
  (bind (_returnvalue_x _returnvalue_y _returnvalue_z) (`KismetMathLibrary.BreakVector` (`self.K2_GetActorLocation`)))
  (bind _returnvalue_x_2 (`KismetMathLibrary.BreakVector` (+ (* (`self.GetActorForwardVector`) 150.0) (`KismetMathLibrary.MakeVector` _returnvalue_x))))
  (if (`self.bCanSpawnPillar`)
    (set `self.bCanSpawnPillar` false)
    (bind _returnvalue (`|SpawnActorFromClass` "/Game/ElementalEchoes/Blueprints/Character/CharacterAbilities/EarthAbilities/BP_StonePillarIndicator.BP_StonePillarIndicator_C" (`KismetMathLibrary.MakeTransform` (`KismetMathLibrary.MakeVector` _returnvalue_x_2 _returnvalue_y (- _returnvalue_z (`CapsuleComponent.GetScaledCapsuleHalfHeight` (`self.CapsuleComponent`))))) "Undefined" "MultiplyWithRoot" null null))
    (return _returnvalue)))

(fn `StopBrace`
  (bind _charactermovement (`self.CharacterMovement`))
  (bind _stoneshield (`self.StoneShield`))
  (set `self.bCanRotate` true)
  (set `CharacterMovementComponent.bOrientRotationToMovement` true (`self.CharacterMovement`))
  (set `CharacterMovementComponent.bUseControllerDesiredRotation` true (`self.CharacterMovement`))
  (set `self.bCanSpawnPillar` true)
  (set `self.bCanJump` true)
  (set `self.bIsBraced` false)
  (set `self.bCanPush/Pull` true)
  (`CharacterMovementComponent.SetMovementMode` _charactermovement "MOVE_Walking" 0)
  (set `CharacterMovementComponent.MaxWalkSpeed` 500.0 _charactermovement)
  (`/Engine/EditorBlueprintResources/StandardMacros.IsValid` _stoneshield
    (:`Is Valid`
      (`self.K2_DestroyActor` _stoneshield)
      (set `self.StoneShield` null))))

(fn `UserConstructionScript`
  (`parent.UserConstructionScript`))