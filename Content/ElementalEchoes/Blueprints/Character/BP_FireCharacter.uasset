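; Fire character for side-on play, with movement, jumping, an interact ability and a chargeable, aimed fireball.
; While the RT ability is ongoing, power charges and a clamped, input-adjusted arc angle sets a launch velocity locked to the XZ plane.
; A debug-drawn path prediction previews the arc plus one mirrored bounce, and triggering spawns BP_FireBall with that velocity.
; LaunchUpwards is uncalled here and PillarSpawn is an empty stub.
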(event `self.ReceiveBeginPlay`
  (`parent.ReceiveBeginPlay`))

(event `EnhancedInput|/Game/Input/Actions/IA_Move`
  (params (ActionValue :type "Vector2D Structure") (ElapsedSeconds :type "Float (double-precision)") (TriggeredSeconds :type "Float (double-precision)") (InputAction :type "InputAction Object Reference" :default "/Game/Input/Actions/IA_Move.IA_Move"))
  ; Movement
  (:`Triggered`
    (set `self.MoveValue` ActionValue_Y)
    (`self.RotateCharacter` ActionValue_Y)
    (`self.Move` ActionValue_Y)))

(event `EnhancedInput|/Game/ElementalEchoes/Blueprints/Controller/InputActions/IA_AbilityRT`
  (params (ActionValue :type Boolean) (ElapsedSeconds :type "Float (double-precision)") (TriggeredSeconds :type "Float (double-precision)") (InputAction :type "InputAction Object Reference" :default "/Game/ElementalEchoes/Blueprints/Controller/InputActions/IA_AbilityRT.IA_AbilityRT"))
  ; Controlling the Projectile Path
  (:`Triggered`
    (`self.LaunchProjectile`))
  (:`Started`
    (set `self.bIsAiming` true)
    (set `self.CurrentPower` 0.0))
  (:`Ongoing`
    (if (`self.bIsAiming`)
      (`self.AddPowerToProjectile`)
      (`self.UpdateTrajectory`))))

(event `EnhancedInput|/Game/ElementalEchoes/Blueprints/Controller/InputActions/IA_MoveProjectilePath`
  (params (ActionValue :type "Vector2D Structure") (ElapsedSeconds :type "Float (double-precision)") (TriggeredSeconds :type "Float (double-precision)") (InputAction :type "InputAction Object Reference" :default "/Game/ElementalEchoes/Blueprints/Controller/InputActions/IA_MoveProjectilePath.IA_MoveProjectilePath"))
  ; Controlling the Projectile Path
  (:`Triggered`
    (if (`self.bIsAiming`)
      (`self.SetArcLimitation` ActionValue_Y))))

(event `EnhancedInput|/Game/ElementalEchoes/Blueprints/Controller/InputActions/IA_BaseAbility`
  (params (ActionValue :type Boolean) (ElapsedSeconds :type "Float (double-precision)") (TriggeredSeconds :type "Float (double-precision)") (InputAction :type "InputAction Object Reference" :default "/Game/ElementalEchoes/Blueprints/Controller/InputActions/IA_BaseAbility.IA_BaseAbility"))
  ; Interact Interface for Destroying Level Actors
  (:`Started`
    (`self.CheckForInteractableObjects`)))

(event `EnhancedInput|/Game/Input/Actions/IA_Jump`
  (params (ActionValue :type Boolean) (ElapsedSeconds :type "Float (double-precision)") (TriggeredSeconds :type "Float (double-precision)") (InputAction :type "InputAction Object Reference" :default "/Game/Input/Actions/IA_Jump.IA_Jump"))
  (:`Started`
    (if (not (`NavMovementInterface.IsFalling` (`self.CharacterMovement`)))
      (`self.Jump`))))

(fn `AddPowerToProjectile`
  (set `self.CurrentPower` (`KismetMathLibrary.FClamp` (+ (`self.CurrentPower`) (* (`GameplayStatics.GetWorldDeltaSeconds`) (`self.ChargeSpeed`))) 0.0 (`self.MaxPower`))))

(fn `LaunchProjectile`
  (bind _returnvalue (`|SpawnActorFromClass` "/Game/ElementalEchoes/Blueprints/Character/CharacterAbilities/FireAbilities/BP_FireBall.BP_FireBall_C" (`KismetMathLibrary.MakeTransform` (`self.K2_GetActorLocation`) (`self.K2_GetActorRotation`)) "Undefined" "MultiplyWithRoot" null null))
  (set `MovementComponent.Velocity` (+ (* (`self.GetActorForwardVector`) 1.0) (`self.LaunchVelocity`)) (`/Game/ElementalEchoes/Blueprints/Character/CharacterAbilities/FireAbilities/BP_FireBall.ProjectileMovement` _returnvalue)))

(fn `LaunchUpwards`
  (if (not (`NavMovementInterface.IsFalling` (`self.CharacterMovement`)))
    (`self.LaunchCharacter` (`KismetMathLibrary.MakeVector` 0.0 0.0 (`self.LaunchHeight`)) false true)))

(fn `PillarSpawn`)

(fn `SetArcLimitation`
  (params (ControllerYAxis :type "Float (double-precision)"))
  (set `self.ArcAngle` (`KismetMathLibrary.FClamp` (+ ControllerYAxis (`self.ArcAngle`)) (`self.MinArcAngle`) (`self.MaxArchAngle`)))
  (`self.UpdateTrajectory`))

(fn `UpdateTrajectory`
  (bind (_returnvalue_x _returnvalue_y _returnvalue_z) (`KismetMathLibrary.BreakVector` (* (+ (* (`self.GetActorForwardVector`) (`KismetMathLibrary.DegCos` (`self.ArcAngle`))) (* (`self.GetActorUpVector`) (`KismetMathLibrary.DegSin` (`self.ArcAngle`)))) (`self.BaseLaunchSpeed`) (`self.CurrentPower`))))
  (bind _output_get (set `self.LaunchVelocity` (`KismetMathLibrary.MakeVector` _returnvalue_x 0.0 _returnvalue_z)))
  (bind (_predictresult _returnvalue) (`GameplayStatics.Blueprint_PredictProjectilePath_Advanced` (make `PredictProjectilePathParams` (`self.K2_GetActorLocation`) (`KismetMathLibrary.MakeVector` (.x _output_get) 0.0 (.z _output_get)) true 5.0 2.0 true "ECC_WorldStatic" _ (`|MakeArray` (`self.GetOwner`) self :!type "Actor Object Reference") 20.0 0.0 "ForOneFrame")))
  (if _returnvalue
    (bind (_bblockinghit _binitialoverlap _time _distance _location _impactpoint _normal _impactnormal) (`GameplayStatics.BreakHitResult` (`.HitResult` (break `PredictProjectilePathResult` _predictresult))))
    (bind (_returnvalue_x_2 _returnvalue_y_2 _returnvalue_z_2) (`KismetMathLibrary.BreakVector` (`KismetMathLibrary.MirrorVectorByNormal` (`self.LaunchVelocity`) _impactnormal)))
    (bind (_returnvalue_x_3 _returnvalue_y_3 _returnvalue_z_3) (`KismetMathLibrary.BreakVector` (* (`KismetMathLibrary.MakeVector` _returnvalue_x_2 _returnvalue_y_2 _returnvalue_z_2) (`self.BounceMultiplier`))))
    (`GameplayStatics.Blueprint_PredictProjectilePath_Advanced` (make `PredictProjectilePathParams` _location (`KismetMathLibrary.MakeVector` _returnvalue_x_3 _returnvalue_y_3 _returnvalue_z_3) false 5.0 2.0 true "ECC_WorldStatic" _ _ 20.0 0.0 "ForOneFrame"))))

(fn `UserConstructionScript`
  (`parent.UserConstructionScript`))