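; Ground-following targeting indicator for the Earth character's stone pillar ability.
; On BeginPlay it caches the character's forward vector and starts a looping timer that steps it along that direction, using downward traces to hover just above the floor.
; At maximum distance it stops and swaps its material.
; The character's spawn event replaces the indicator with a BP_StonePillar at its position, slightly lowered.
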(event `self.ReceiveBeginPlay`
  (bind _returnvalue (`GameplayStatics.GetActorOfClass` "/Game/ElementalEchoes/Blueprints/Character/BP_EarthCharacter.BP_EarthCharacter_C"))
  (bind _output_get (set `self.EarthCharacter` _returnvalue))
  (set `self.PlayersForwardVector` (`self.GetActorForwardVector` _output_get))
  (`KismetSystemLibrary.K2_SetTimerDelegate` (delegate `Move`) 0.02 true)
  (add `/Game/ElementalEchoes/Blueprints/Character/BP_EarthCharacter.SpawnStonePillar` _returnvalue (delegate `SpawnStonePillar`)))

(event `SpawnStonePillar`
  (`self.SpawnPillar`))

(event `Move`
  (`self.TranslateAcrossFloor`))

(event `SpawnPillar`
  (bind _returnvalue (`self.GetTransform`))
  (`|SpawnActorFromClass` "/Game/ElementalEchoes/Blueprints/Character/CharacterAbilities/EarthAbilities/BP_StonePillar.BP_StonePillar_C" (`KismetMathLibrary.MakeTransform` (`KismetMathLibrary.MakeVector` (.x (.location _returnvalue)) (.y (.location _returnvalue)) (- (.z (.location _returnvalue)) 10.0)) (.rotation _returnvalue)) "Undefined" "MultiplyWithRoot" null null)
  (`self.K2_DestroyActor`))

(fn `BP_StonePillarIndicator_AutoGenFunc`
  (params (DestroyedActor :type "Actor Object Reference")))

(fn `KeepCloseToFloor`
  (returns (`Z Value of Floor` :type "Float (double-precision)"))
  (bind (_returnvalue_x _returnvalue_y _returnvalue_z) (`KismetMathLibrary.BreakVector` (`self.K2_GetActorLocation`)))
  (bind _outhit (`KismetSystemLibrary.LineTraceSingle` (`self.K2_GetActorLocation`) (`KismetMathLibrary.MakeVector` _returnvalue_x _returnvalue_y (- _returnvalue_z 100.0)) "TraceTypeQuery3"))
  (bind (_bblockinghit _binitialoverlap _time _distance _location) (`GameplayStatics.BreakHitResult` _outhit))
  (if _bblockinghit
    (return (+ (.z _location) 10.0))))

(fn `SpawnPillar1`
  (bind _returnvalue (`self.GetTransform`))
  (bind _returnvalue_2 (`|SpawnActorFromClass` "/Game/ElementalEchoes/Blueprints/Character/CharacterAbilities/EarthAbilities/BP_StonePillar.BP_StonePillar_C" (`KismetMathLibrary.MakeTransform` (`KismetMathLibrary.MakeVector` (.x (.location _returnvalue)) (.y (.location _returnvalue)) (- (.z (.location _returnvalue)) 10.0)) (.rotation _returnvalue)) "Undefined" "MultiplyWithRoot" null null))
  (add `self.OnDestroyed` _returnvalue_2 (`|CreateDelegate` :!event `BP_StonePillarIndicator_AutoGenFunc`))
  (`self.K2_DestroyActor`))

(fn `TranslateAcrossFloor`
  (locals (Currentlocation :type "Vector Structure") (Step :type "Vector Structure") (NewLocation :type "Vector Structure"))
  (bind (_newlocation_x _newlocation_y) (`KismetMathLibrary.BreakVector` (`local.NewLocation`)))
  (set `local.Currentlocation` (`self.K2_GetActorLocation`))
  (set `local.Step` (* (`self.DistaceToMove`) (`self.PlayersForwardVector`)))
  (set `local.NewLocation` (+ (`local.Step`) (`local.Currentlocation`)))
  (if (>= (`self.CurrentDistance`) (`self.MaxDistance`))
    (`PrimitiveComponent.SetMaterial` (`self.Indicator`) 0 "/Game/ThirdPerson/MI_ThirdPersonColWay.MI_ThirdPersonColWay")
    (else
      (bind _z_value_of_floor (`self.KeepCloseToFloor`))
      (`self.K2_SetActorLocation` (`KismetMathLibrary.MakeVector` _newlocation_x _newlocation_y _z_value_of_floor))
      (set `self.CurrentDistance` (+ (`self.CurrentDistance`) (`self.DistaceToMove`))))))

(fn `UserConstructionScript`)