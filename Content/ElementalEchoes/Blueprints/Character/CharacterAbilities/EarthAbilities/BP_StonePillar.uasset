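; Earth ability actor for a stone pillar that rises on spawn and launches fire characters upward.
; A timeline raises it by adding its curve value to the current Z each update, so movement accumulates.
; When the timeline finishes, every BP_FireCharacter overlapping the sphere gets LaunchUpwards.
; A three-second delay, started on BeginPlay alongside the rise, destroys the pillar.
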(event `self.ReceiveBeginPlay`
  (`self.RaisePillar`)
  (`self.HandleDestruction`))

(event `RaisePillar`
  (bind (_returnvalue_x _returnvalue_y _returnvalue_z) (`KismetMathLibrary.BreakVector` (`self.K2_GetActorLocation`)))
  (bind (_direction _pillarzlocation) (`Timeline|PillarControl`)
    (:`Update`
      (`self.K2_SetActorLocation` (`KismetMathLibrary.MakeVector` _returnvalue_x _returnvalue_y (+ _returnvalue_z _pillarzlocation))))
    (:`Finished`
      (`self.TryLaunchPlayer`))))

(event `HandleDestruction`
  (`KismetSystemLibrary.Delay` 3.0)
  (`self.K2_DestroyActor`))

(fn `TryLaunchPlayer`
  (for _array_element (`PrimitiveComponent.GetOverlappingActors` (`self.Sphere`) "/Game/ElementalEchoes/Blueprints/Character/BP_FireCharacter.BP_FireCharacter_C")
    (`/Engine/EditorBlueprintResources/StandardMacros.IsValid` _array_element
      (:`Is Valid`
        (bind _asbp_fire_character (cast `/Game/ElementalEchoes/Blueprints/Character/BP_FireCharacter` _array_element))
        (`/Game/ElementalEchoes/Blueprints/Character/BP_FireCharacter.LaunchUpwards` _asbp_fire_character)))))

(fn `UserConstructionScript`)