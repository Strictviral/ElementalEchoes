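; Puzzle gate actor that raises when its required objects become active and can close again.
; On BeginPlay it counts the OpenObjects and binds to their active and inactive events, plus each lever's activate event.
; A remaining-objects counter triggers opening at zero and closing when it returns to one.
; Separate timelines lerp the mesh's Z up or down from the actor's location, applied as a relative location.
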(event `self.ReceiveBeginPlay`
  (`self.InitializeObjects`)
  (`self.InitalizeLevers`))

(event `AddAndCheckForOpenObjectsRemaining`
  ; Check to see If the Gate can Open
  (bind _result (`/Engine/EditorBlueprintResources/StandardMacros.DecrementFloat` (`self.OpenObjectsNeeded`))
    (:`  `
      (if (<= _result 0.0)
        (`self.OpenGate`)))))

(event `SubtractAndCheckForOpenObjectsRemaining`
  ; Check to close the gate
  (bind _result (`/Engine/EditorBlueprintResources/StandardMacros.IncrementFloat` (`self.OpenObjectsNeeded`))
    (:`  `
      (if (== _result 1.0)
        (`self.CloseGate`)))))

(event `OpenGate`
  (bind (_returnvalue_x _returnvalue_y _returnvalue_z) (`KismetMathLibrary.BreakVector` (`self.K2_GetActorLocation`)))
  (bind (_direction _gateopenup) (`Timeline|Timeline`)
    (:`Update`
      (`SceneComponent.K2_SetRelativeLocation` (`self.GateMesh`) (`KismetMathLibrary.MakeVector` _returnvalue_x _returnvalue_y (`KismetMathLibrary.Lerp` _returnvalue_z (+ _returnvalue_z 5.0) _gateopenup)) false false))))

(event `CloseGate`
  (bind (_returnvalue_x _returnvalue_y _returnvalue_z) (`KismetMathLibrary.BreakVector` (`self.K2_GetActorLocation`)))
  (bind (_direction _gateopenup) (`Timeline|Timeline_0`)
    (:`Update`
      (`SceneComponent.K2_SetRelativeLocation` (`self.GateMesh`) (`KismetMathLibrary.MakeVector` _returnvalue_x _returnvalue_y (`KismetMathLibrary.Lerp` _returnvalue_z (- _returnvalue_z 5.0) _gateopenup)) false false))))

(fn `InitalizeLevers`
  (for _array_element (`self.Levers`)
    (add `/Game/ElementalEchoes/Blueprints/PuzzleActors/BP_Lever.LeverActivate` _array_element (`|CreateDelegate` :!event `OpenGate`))))

(fn `InitializeObjects`
  (for _array_element (`self.OpenObjects`)
    (bind _result (`/Engine/EditorBlueprintResources/StandardMacros.IncrementFloat` (`self.OpenObjectsFound`))
      (:`  `
        (set `self.OpenObjectsNeeded` _result)
        (`/Engine/EditorBlueprintResources/StandardMacros.IsValid` _array_element
          (:`Is Valid`
            (add `/Game/ElementalEchoes/Blueprints/PuzzleActors/BP_OpenObjects.ObjectActive` _array_element (`|CreateDelegate` :!event `AddAndCheckForOpenObjectsRemaining`))
            (add `/Game/ElementalEchoes/Blueprints/PuzzleActors/BP_OpenObjects.ObjectsInactive` _array_element (`|CreateDelegate` :!event `SubtractAndCheckForOpenObjectsRemaining`))))))))

(fn `UserConstructionScript`)