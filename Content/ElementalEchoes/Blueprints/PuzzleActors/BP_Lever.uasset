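; BP_Lever is an interactable puzzle lever that toggles on and off and broadcasts LeverActivate on each use.
; Interact runs HandleOnOff, which fires the dispatcher, plays or reverses the Turn timeline to rotate the handle, then flips IsActive.
; A sphere overlap shows an animated WBP_LevelPrompt through a widget component for Player-tagged actors, hiding it on interaction or shortly after they leave.
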(event `/Game/ElementalEchoes/Blueprints/Interface/BPI_Interact.Interact`
  (params (CharacterName :type String))
  (`self.HandleOn/Off`)
  (`self.Hide Level Prompt Widget`))

(event `TurnLever`
  (if (not (`self.bIsActive`))
    (bind (_direction _leverrotation) (`Timeline|Turn` :!label _label)
      (:`Update`
        (`SceneComponent.K2_SetRelativeRotation` (`self.LeverHandle`) (`KismetMathLibrary.RLerp` (struct :`Pitch` 70.0) (struct) _leverrotation) false false)))
    (else
      (goto _label :!via `Reverse`))))

(event `self.Sphere.OnComponentBeginOverlap`
  (params (OverlappedComponent :type "PrimitiveComponent Object Reference") (OtherActor :type "Actor Object Reference") (OtherComp :type "PrimitiveComponent Object Reference") (OtherBodyIndex :type Integer) (bFromSweep :type Boolean) (SweepResult :type "HitResult Structure (by ref)"))
  (bind _widget (`self.Widget`))
  (if (`self.ActorHasTag` OtherActor "Player")
    (if (not (`self.bIs UI on Screen?`))
      (bind _returnvalue (`|CreateWidget` "/Game/ElementalEchoes/Blueprints/UI/WBP_LevelPrompt.WBP_LevelPrompt_C"))
      (bind _output_get (set `self.Widget LevelPrompt` _returnvalue))
      (`/Game/ElementalEchoes/Blueprints/UI/WBP_LevelPrompt.Set Interaction Type Text` _output_get (`self.Interact Type`))
      (`WidgetComponent.SetWidget` _widget _output_get)
      (`SceneComponent.SetVisibility` _widget true false)
      (`UserWidget.PlayAnimation` _output_get (`/Game/ElementalEchoes/Blueprints/UI/WBP_LevelPrompt.Show` _output_get) 0.0 1 "Forward" 1.0 false)
      (set `self.bIs UI on Screen?` true))))

(event `self.Sphere.OnComponentEndOverlap`
  (params (OverlappedComponent :type "PrimitiveComponent Object Reference") (OtherActor :type "Actor Object Reference") (OtherComp :type "PrimitiveComponent Object Reference") (OtherBodyIndex :type Integer))
  (if (`self.ActorHasTag` OtherActor "Player")
    (if (`self.bIs UI on Screen?`)
      (`KismetSystemLibrary.Delay` 0.5)
      (`self.Hide Level Prompt Widget`))))

(event `Hide Level Prompt Widget`
  (bind _widget_levelprompt (`self.Widget LevelPrompt`))
  (if (`self.bIs UI on Screen?`)
    (`UserWidget.PlayAnimation` _widget_levelprompt (`/Game/ElementalEchoes/Blueprints/UI/WBP_LevelPrompt.Hide` _widget_levelprompt) 0.0 1 "Forward" 1.0 false)
    (`KismetSystemLibrary.Delay` 0.35)
    (`Widget.RemoveFromParent` (`self.Widget LevelPrompt`))
    (`SceneComponent.SetVisibility` (`self.Widget`) false false)
    (set `self.bIs UI on Screen?` false)))

(fn `HandleOn/Off`
  (if (not (`self.bIsActive`))
    (`self.LeverActivate`)
    (`self.TurnLever`)
    (set `self.bIsActive` true)
    (else
      (`self.LeverActivate`)
      (`self.TurnLever`)
      (set `self.bIsActive` false))))

(fn `UserConstructionScript`
  (`parent.UserConstructionScript`))