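; BP_Torch is a puzzle lantern that the player's fire can light by hitting it with a BP_FireBall.
; An overlap on its sphere, while unlit, tells the fireball to handle its destruction, runs LightLantern, then calls CallObjectActive to signal activation.
; LightLantern sets the lit flag, raises the point light intensity and activates the Niagara effect; nothing here unlights it.
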(event `self.Sphere.OnComponentBeginOverlap`
  (params (OverlappedComponent :type "PrimitiveComponent Object Reference") (OtherActor :type "Actor Object Reference") (OtherComp :type "PrimitiveComponent Object Reference") (OtherBodyIndex :type Integer) (bFromSweep :type Boolean) (SweepResult :type "HitResult Structure (by ref)"))
  (if (not (`self.bIsLit`))
    (bind _asbp_fire_ball (cast `/Game/ElementalEchoes/Blueprints/Character/CharacterAbilities/FireAbilities/BP_FireBall` OtherActor))
    (`/Game/ElementalEchoes/Blueprints/Character/CharacterAbilities/FireAbilities/BP_FireBall.HandleDestruction` _asbp_fire_ball)
    (`self.LightLantern`)
    (`self.ObjectActive`)))

(fn `InitalizeLantern`
  (set `self.StaticMeshLantern` (`self.LanternStaticMesh`)))

(fn `LightLantern`
  (set `self.bIsLit` true)
  (`LightComponent.SetIntensity` (`self.PointLight`) (`self.LightIntensity`))
  (`ActorComponent.Activate` (`self.Niagara`) false))

(fn `UserConstructionScript`)