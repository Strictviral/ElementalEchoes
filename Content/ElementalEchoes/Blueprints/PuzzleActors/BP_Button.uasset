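; BP_Button is an interactable puzzle button that signals other objects to turn on and off.
; Interact runs HandleOnOff, which, if inactive, calls Activate then Deactivate, setting IsActive and firing CallObjectActive and CallObjectsInactive respectively.
; Deactivate first triggers DelayTimer, but that event's three-second Delay has nothing after it, so deactivation follows activation immediately.
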(event `/Game/ElementalEchoes/Blueprints/Interface/BPI_Interact.Interact`
  ; Interact Interface to Turn On/off
  (`self.HandleOn/Off`))

(event `DelayTimer`
  ; Delay to Be used in Functions
  (`KismetSystemLibrary.Delay` 3.0))

(fn `Activate`
  (`self.ObjectActive`)
  (set `self.bIsActive` true))

(fn `Deactivate`
  (`self.DelayTimer`)
  (`self.ObjectsInactive`)
  (set `self.bIsActive` false))

(fn `HandleOn/Off`
  (if (not (`self.bIsActive`))
    (`self.Activate`)
    (`self.Deactivate`)))

(fn `UserConstructionScript`)