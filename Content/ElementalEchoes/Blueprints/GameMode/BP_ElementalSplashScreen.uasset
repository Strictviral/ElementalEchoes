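; Splash screen Blueprint for Elemental Echoes that shows the opening splash and then moves the game to the main menu level.
; On BeginPlay it sets the default sound mix, adds the splash widget to the viewport and starts a timer.
; When the timer fires, it plays the widget's fade-out, waits briefly and opens Lvl_Menu.
; A separate helper, not called here, adds the UI input mapping context to the first player controller found and returns it.
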(event `self.ReceiveBeginPlay`
  (`|ExecutionSequence`
    (:`then_0`
      (`GameplayStatics.SetBaseSoundMix` "/Game/ElementalEchoes/Blueprints/Audio/Classes/SCM_DefaultSound.SCM_DefaultSound"))
    (:`then_1`
      (bind _returnvalue (`|CreateWidget` "/Game/ElementalEchoes/Blueprints/UI/WBP_Splash.WBP_Splash_C"))
      (bind _output_get (set `self.Splash Widget` _returnvalue))
      (`UserWidget.AddToViewport` _output_get 0)
      (bind _returnvalue_2 (`KismetSystemLibrary.K2_SetTimerDelegate` (delegate `MovetoMain Menu`) 7.5))
      (set `self.Timer Handle` _returnvalue_2))))

(event `MovetoMain Menu`
  (bind _splash_widget (`self.Splash Widget`))
  (`UserWidget.PlayAnimation` _splash_widget (`/Game/ElementalEchoes/Blueprints/UI/WBP_Splash.FadeOut` _splash_widget) 0.0 1 "Forward" 1.0 false)
  (`KismetSystemLibrary.Delay` 1.0)
  (`GameplayStatics.OpenLevel` "Lvl_Menu"))

(fn `List of Controllers`
  (returns (Controllers :type "PlayerController Object Reference"))
  (bind _outactors (`GameplayStatics.GetAllActorsOfClass` "/Script/Engine.PlayerController"))
  (for _array_element _outactors
    (`EnhancedInputSubsystemInterface.AddMappingContext` (pcsubsystem `EnhancedInputLocalPlayerSubsystem` _array_element) "/Game/ElementalEchoes/Blueprints/Controller/IMC_ElementalUI.IMC_ElementalUI" 0 (struct))
    (return _array_element)))

(fn `UserConstructionScript`)