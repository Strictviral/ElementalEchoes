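; BP_ElementalMenu sets up the main menu for Elemental Echoes, including its UI input and default sound mix.
; On BeginPlay, ListOfControllers searches for player controllers, adds the IMC_ElementalUI Enhanced Input mapping context, and returns from inside the loop, so only the first controller is handled.
; It then creates WBP_MainMenu, adds it to the viewport, initialises it with that controller and sets SCM_DefaultSound as the base mix.
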(event `self.ReceiveBeginPlay`
  (`|ExecutionSequence`
    (:`then_0`
      (bind _controllers (`self.List of Controllers`))
      (set `self.Controllers` _controllers))
    (:`then_1`
      (bind _returnvalue (`|CreateWidget` "/Game/ElementalEchoes/Blueprints/UI/WBP_MainMenu.WBP_MainMenu_C"))
      (`UserWidget.AddToViewport` _returnvalue 0)
      (bind _output_get (set `self.Main Menu Widget` _returnvalue))
      (`/Game/ElementalEchoes/Blueprints/UI/WBP_MainMenu.Initialise` _output_get (`self.Controllers`))
      (`GameplayStatics.SetBaseSoundMix` "/Game/ElementalEchoes/Blueprints/Audio/Classes/SCM_DefaultSound.SCM_DefaultSound"))))

(fn `List of Controllers`
  (returns (Controllers :type "PlayerController Object Reference"))
  (bind _outactors (`GameplayStatics.GetAllActorsOfClass` "/Script/Engine.PlayerController"))
  (for _array_element _outactors
    (`EnhancedInputSubsystemInterface.AddMappingContext` (pcsubsystem `EnhancedInputLocalPlayerSubsystem` _array_element) "/Game/ElementalEchoes/Blueprints/Controller/IMC_ElementalUI.IMC_ElementalUI" 0 (struct))
    (return _array_element)))

(fn `UserConstructionScript`)