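; Game mode for Elemental Echoes local co-op that creates a second local player, spawns Fire and Earth characters at tagged PlayerStarts and possesses them by controller ID.
; Character events update PlayerLives, which counts dead players despite its name.
; When it reaches two, movement stops, input switches to the UI mapping context and a death screen appears.
; The screen's checkpoint event is bound, and RespawnPlayers revives both characters and restores gameplay input.
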(event `self.ReceiveBeginPlay`
  (if (not (> (`GameplayStatics.GetNumLocalPlayerControllers`) 1))
    (`GameplayStatics.CreatePlayer` -1))
  (bind _returnvalue (`GameplayStatics.GetActorOfClass` "/Game/ElementalEchoes/Blueprints/Camera/BP_SharedDynamicCamera.BP_SharedDynamicCamera_C"))
  (set `self.DynamicCamera` _returnvalue)
  (`GameplayStatics.SetBaseSoundMix` "/Game/ElementalEchoes/Blueprints/Audio/Classes/SCM_DefaultSound.SCM_DefaultSound"))

(event `self.K2_PostLogin`
  (params (NewPlayer :type "PlayerController Object Reference"))
  ; Assign Controllers
  (if (== (`GameplayStatics.GetPlayerControllerID` NewPlayer) 0)
    (bind _asbp_elemental_controller (cast `/Game/ElementalEchoes/Blueprints/Controller/BP_ElementalController` NewPlayer))
    (`self.SpawnFireCharacter`)
    (`Controller.Possess` _asbp_elemental_controller (`self.FireCharacter`))
    (`EnhancedInputSubsystemInterface.AddMappingContext` (pcsubsystem `EnhancedInputLocalPlayerSubsystem` _asbp_elemental_controller) "/Game/ElementalEchoes/Blueprints/Controller/IMC_ElementalMappingContext.IMC_ElementalMappingContext" 0 (struct))
    (bind _asbp_base_character (cast `/Game/ElementalEchoes/Blueprints/Character/BP_BaseCharacter` (`Controller.K2_GetPawn` _asbp_elemental_controller)))
    (add `/Game/ElementalEchoes/Blueprints/Character/BP_BaseCharacter.AddDeadPlayers` _asbp_base_character (`|CreateDelegate` :!event `AddDeadPlayersAndCheck`))
    (add `/Game/ElementalEchoes/Blueprints/Character/BP_BaseCharacter.RemoveDeadPlayers` _asbp_base_character (`|CreateDelegate` :!event `RemoveDeadPlayers`))
    (else
      (bind _asbp_elemental_controller_2 (cast `/Game/ElementalEchoes/Blueprints/Controller/BP_ElementalController` NewPlayer))
      (`self.SpawnEarthCharacter`)
      (`Controller.Possess` _asbp_elemental_controller_2 (`self.EarthCharacter`))
      (`EnhancedInputSubsystemInterface.AddMappingContext` (pcsubsystem `EnhancedInputLocalPlayerSubsystem` _asbp_elemental_controller_2) "/Game/ElementalEchoes/Blueprints/Controller/IMC_ElementalMappingContext.IMC_ElementalMappingContext" 0 (struct))
      (bind _asbp_base_character_2 (cast `/Game/ElementalEchoes/Blueprints/Character/BP_BaseCharacter` (`Controller.K2_GetPawn` _asbp_elemental_controller_2)))
      (add `/Game/ElementalEchoes/Blueprints/Character/BP_BaseCharacter.AddDeadPlayers` _asbp_base_character_2 (`|CreateDelegate` :!event `AddDeadPlayersAndCheck`))
      (add `/Game/ElementalEchoes/Blueprints/Character/BP_BaseCharacter.RemoveDeadPlayers` _asbp_base_character_2 (`|CreateDelegate` :!event `RemoveDeadPlayers`)))))

(event `SpawnFireCharacter`
  ; Spawn Fire Character Correctly
  (bind _firestarttransform (`self.GetPlayerFireStart`))
  (bind _returnvalue (`|SpawnActorFromClass` "/Game/ElementalEchoes/Blueprints/Character/BP_FireCharacter.BP_FireCharacter_C" (`KismetMathLibrary.MakeTransform` (.location _firestarttransform) (.rotation _firestarttransform)) "Undefined" "MultiplyWithRoot" null null))
  (set `self.FireCharacter` _returnvalue))

(event `SpawnEarthCharacter`
  ; Spawn Earth Character Correctly
  (bind _earthstarttransform (`self.GetPlayerEarthStart`))
  (bind _returnvalue (`|SpawnActorFromClass` "/Game/ElementalEchoes/Blueprints/Character/BP_EarthCharacter.BP_EarthCharacter_C" (`KismetMathLibrary.MakeTransform` (.location _earthstarttransform) (.rotation _earthstarttransform)) "Undefined" "MultiplyWithRoot" null null))
  (set `self.EarthCharacter` _returnvalue))

(fn `AddDeadPlayersAndCheck`
  (bind _result (`/Engine/EditorBlueprintResources/StandardMacros.IncrementInt` (`self.PlayerLives`))
    (:`  `
      (`KismetSystemLibrary.PrintString` (`KismetStringLibrary.Concat_StrStr` "Number of Players Dead: " (`KismetStringLibrary.Conv_IntToString` _result)))
      (`self.CheckForGameEnd`))))

(fn `CheckForGameEnd`
  (if (== (`self.PlayerLives`) 2)
    (`self.LoopThroughLocalControllersEnterUIMode`)
    (bind _returnvalue (`|CreateWidget` "/Game/ElementalEchoes/Blueprints/UI/WBP_DeathScreen.WBP_DeathScreen_C" (`GameplayStatics.GetPlayerController` 0)))
    (`UserWidget.AddToViewport` _returnvalue 0)
    (set `self.Death Screen` _returnvalue)
    (`/Game/ElementalEchoes/Blueprints/UI/WBP_DeathScreen.Initialise` _returnvalue (`GameplayStatics.GetPlayerController` 0))
    (add `/Game/ElementalEchoes/Blueprints/UI/WBP_DeathScreen.E_LoadMostRecentCheckpoint` _returnvalue (`|CreateDelegate` :!event `RespawnPlayers`))))

(fn `GetPlayerEarthStart`
  (returns (EarthStartTransform :type "Transform Structure"))
  (bind _outactors (`GameplayStatics.GetAllActorsOfClass` "/Script/Engine.PlayerStart"))
  (for _array_element _outactors
    (if (== (`PlayerStart.PlayerStartTag` _array_element) "EarthStart")
      (return (`self.GetTransform` _array_element)))))

(fn `GetPlayerFireStart`
  (returns (FireStartTransform :type "Transform Structure"))
  (bind _outactors (`GameplayStatics.GetAllActorsOfClass` "/Script/Engine.PlayerStart"))
  (for _array_element _outactors
    (if (== (`PlayerStart.PlayerStartTag` _array_element) "FireStart")
      (return (`self.GetTransform` _array_element)))))

(fn `LoopThroughLocalControllersEnterUIMode`
  (bind _outactors (`GameplayStatics.GetAllActorsOfClass` "/Script/Engine.PlayerController"))
  (for _array_element _outactors
    (`|ExecutionSequence`
      (:`then_0`
        (bind _returnvalue (pcsubsystem `EnhancedInputLocalPlayerSubsystem` _array_element))
        (`EnhancedInputSubsystemInterface.AddMappingContext` _returnvalue "/Game/ElementalEchoes/Blueprints/Controller/IMC_ElementalUI.IMC_ElementalUI" 1 (struct))
        (`KismetSystemLibrary.PrintString` "Mapping to UI")
        (`EnhancedInputSubsystemInterface.RemoveMappingContext` _returnvalue "/Game/ElementalEchoes/Blueprints/Controller/IMC_ElementalMappingContext.IMC_ElementalMappingContext" (struct)))
      (:`then_1`
        (bind _asbp_base_character (cast `/Game/ElementalEchoes/Blueprints/Character/BP_BaseCharacter` (`Controller.K2_GetPawn` _array_element)))
        (`ActorComponent.SetActive` (`Pawn.GetMovementComponent` _asbp_base_character) false false)
        (set `/Game/ElementalEchoes/Blueprints/Character/BP_BaseCharacter.bHasGameEnded` true _asbp_base_character)))))

(fn `RemoveDeadPlayers`
  (`/Engine/EditorBlueprintResources/StandardMacros.DecrementInt` (`self.PlayerLives`)))

(fn `RespawnPlayers`
  (`/Game/ElementalEchoes/Blueprints/Character/BP_BaseCharacter.Respawn` (`self.FireCharacter`))
  (`/Game/ElementalEchoes/Blueprints/Character/BP_BaseCharacter.Respawn` (`self.EarthCharacter`))
  (bind _outactors (`GameplayStatics.GetAllActorsOfClass` "/Script/Engine.PlayerController"))
  (for _array_element _outactors
    (bind _returnvalue (pcsubsystem `EnhancedInputLocalPlayerSubsystem` _array_element))
    (`EnhancedInputSubsystemInterface.AddMappingContext` _returnvalue "/Game/ElementalEchoes/Blueprints/Controller/IMC_ElementalMappingContext.IMC_ElementalMappingContext" 0 (struct))
    (`KismetSystemLibrary.PrintString` "Mapping to Game" true true (struct :`R` 1.0 :`B` 0.361135 :`A` 1.0))
    (`EnhancedInputSubsystemInterface.RemoveMappingContext` _returnvalue "/Game/ElementalEchoes/Blueprints/Controller/IMC_ElementalUI.IMC_ElementalUI" (struct))
    (`Widget.RemoveFromParent` (`self.Death Screen`))))

(fn `UserConstructionScript`)