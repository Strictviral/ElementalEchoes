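; KillingFloorBorder is a level actor that acts as a kill zone for characters.
; When an actor overlaps its Box, it casts to BP_BaseCharacter and calls HandleDeath on that character.
; BeginPlay also caches the fire and earth characters as Player1 and Player2, the latter after a short delay, but only a disconnected per-player death branch uses them.
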(event `self.ReceiveBeginPlay`
  (bind _returnvalue (`GameplayStatics.GetActorOfClass` "/Game/ElementalEchoes/Blueprints/Character/BP_FireCharacter.BP_FireCharacter_C"))
  (set `self.Player1` _returnvalue)
  (`KismetSystemLibrary.Delay` 0.2)
  (bind _returnvalue_2 (`GameplayStatics.GetActorOfClass` "/Game/ElementalEchoes/Blueprints/Character/BP_EarthCharacter.BP_EarthCharacter_C"))
  (set `self.Player2` _returnvalue_2))

(event `self.Box.OnComponentBeginOverlap`
  (params (OverlappedComponent :type "PrimitiveComponent Object Reference") (OtherActor :type "Actor Object Reference") (OtherComp :type "PrimitiveComponent Object Reference") (OtherBodyIndex :type Integer) (bFromSweep :type Boolean) (SweepResult :type "HitResult Structure (by ref)"))
  (bind _asbp_base_character (cast `/Game/ElementalEchoes/Blueprints/Character/BP_BaseCharacter` OtherActor))
  (`/Game/ElementalEchoes/Blueprints/Character/BP_BaseCharacter.HandleDeath` _asbp_base_character))

(fn `UserConstructionScript`)