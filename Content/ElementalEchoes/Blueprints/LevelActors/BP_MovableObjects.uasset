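; BP_MovableObjects is a stone that the Earth character can push and pull.
; Interacting asks the cached Earth character to attach if it is idle and not falling, otherwise to detach.
; A sphere overlap shows an animated prompt widget, which hides on attach or shortly after leaving.
; Speed/Direction moves the mesh along its forward vector by a signed speed, using VInterpTo without sweep.
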(event `self.ReceiveBeginPlay`
  (`KismetSystemLibrary.Delay` 0.5)
  (bind _returnvalue (`GameplayStatics.GetActorOfClass` "/Game/ElementalEchoes/Blueprints/Character/BP_EarthCharacter.BP_EarthCharacter_C"))
  (set `self.EarthCharacterRef` _returnvalue))

(event `/Game/ElementalEchoes/Blueprints/Interface/BPI_Interact.Interact`
  (params (CharacterName :type String))
  (bind _earthcharacterref (`self.EarthCharacterRef`))
  ; Interact Event For Pushing and Pulling
  (switch `string` CharacterName
    (:`Tremor`
      (if (and (not (`/Game/ElementalEchoes/Blueprints/Character/BP_EarthCharacter.bIsInteracting` _earthcharacterref)) (not (`NavMovementInterface.IsFalling` (`Pawn.GetMovementComponent` _earthcharacterref))))
        (`/Game/ElementalEchoes/Blueprints/Character/BP_EarthCharacter.CheckandAttachMovingObject` (`self.EarthCharacterRef`))
        (`self.Hide Level Prompt Widget`)
        (else
          (`/Game/ElementalEchoes/Blueprints/Character/BP_EarthCharacter.DetachFromMovingObject` (`self.EarthCharacterRef`)))))))

(event `self.Sphere.OnComponentBeginOverlap`
  (params (OverlappedComponent :type "PrimitiveComponent Object Reference") (OtherActor :type "Actor Object Reference") (OtherComp :type "PrimitiveComponent Object Reference") (OtherBodyIndex :type Integer) (bFromSweep :type Boolean) (SweepResult :type "HitResult Structure (by ref)"))
  (bind _widget (`self.Widget`))
  (if (== OtherActor (`self.EarthCharacterRef`))
    (bind _returnvalue (`|CreateWidget` "/Game/ElementalEchoes/Blueprints/UI/WBP_LevelPrompt.WBP_LevelPrompt_C"))
    (bind _output_get (set `self.Widget LevelPrompt` _returnvalue))
    (`WidgetComponent.SetWidget` _widget _output_get)
    (`SceneComponent.SetVisibility` _widget true false)
    (`UserWidget.PlayAnimation` _output_get (`/Game/ElementalEchoes/Blueprints/UI/WBP_LevelPrompt.Show` _output_get) 0.0 1 "Forward" 1.0 false)))

(event `self.Sphere.OnComponentEndOverlap`
  (params (OverlappedComponent :type "PrimitiveComponent Object Reference") (OtherActor :type "Actor Object Reference") (OtherComp :type "PrimitiveComponent Object Reference") (OtherBodyIndex :type Integer))
  (if (== OtherActor (`self.EarthCharacterRef`))
    (`KismetSystemLibrary.Delay` 1.0)
    (`self.Hide Level Prompt Widget`)))

(event `Hide Level Prompt Widget`
  (bind _widget_levelprompt (`self.Widget LevelPrompt`))
  (`UserWidget.PlayAnimation` _widget_levelprompt (`/Game/ElementalEchoes/Blueprints/UI/WBP_LevelPrompt.Hide` _widget_levelprompt) 0.0 1 "Forward" 1.0 false)
  (`KismetSystemLibrary.Delay` 0.35)
  (`Widget.RemoveFromParent` (`self.Widget LevelPrompt`))
  (`SceneComponent.SetVisibility` (`self.Widget`) false false))

(fn `UserConstructionScript`)