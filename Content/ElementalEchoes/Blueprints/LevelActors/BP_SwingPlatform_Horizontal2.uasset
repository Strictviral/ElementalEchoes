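; A horizontal swing platform level actor that rotates open when all of its linked objects, such as pressure plates, are active.
; BeginPlay binds to each linked object's active and inactive events and to lever activation, then compares a running active count against the number linked.
; A timeline lerps the platform's roll a quarter turn with sound cues, destroying StaticMesh2 as it updates, and reverses when the count falls short.
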(event `self.ReceiveBeginPlay`
  (bind (_relativerotation_roll _relativerotation_pitch _relativerotation_yaw) (`KismetMathLibrary.BreakRotator` (`SceneComponent.RelativeRotation` (`self.Platform`))))
  ; Initialized and find all actors
  (set `self.Return Value Y (Pitch)` _relativerotation_pitch)
  (set `self.Return Value Z (Yaw)` _relativerotation_yaw)
  (for _array_element (`self.OpenObjects`)
    (`/Engine/EditorBlueprintResources/StandardMacros.IncrementFloat` (`self.AmountofObjectsFound`)
      (:`  `
        (add `/Game/ElementalEchoes/Blueprints/PuzzleActors/BP_OpenObjects.ObjectActive` _array_element (delegate `SwingPlatformOpen`))
        (add `/Game/ElementalEchoes/Blueprints/PuzzleActors/BP_OpenObjects.ObjectsInactive` _array_element (delegate `SwingPlatformClosed`)))))
  (for _array_element_2 (`self.Lever`)
    (add `/Game/ElementalEchoes/Blueprints/PuzzleActors/BP_Lever.LeverActivate` _array_element_2 (`|CreateDelegate` :!event `SwingPlatformActive`))))

(event `SwingPlatformOpen`
  ; Initialized and find all actors
  (`self.IncreasePressurePlateActive`)
  (`self.CheckPlatforms`))

(event `SwingPlatformClosed`
  ; Initialized and find all actors
  (`self.DecresePressurePlatesActive`)
  (`self.CheckPlatforms`))

(event `CheckPlatforms`
  ; Check to see if Pressur plates are active
  (if (>= (`self.AmountofActiveObjects`) (`self.AmountofObjectsFound`))
    (`self.SwingPlatformActive`)
    (else
      (`self.SwingPlatformUnactive`))))

(event `SwingPlatformActive`
  ; Animation for Platform Swing
  (`GameplayStatics.PlaySound2D` "/Game/ElementalEchoes/Blueprints/Audio/Cues/swing_platform_Cue.swing_platform_Cue" 1.0 1.0 0.0 null null)
  (bind (_direction _swing) (`Timeline|Timeline` :!label _label)
    (:`Update`
      (`SceneComponent.K2_SetRelativeRotation` (`self.Platform`) (`KismetMathLibrary.MakeRotator` (`KismetMathLibrary.Lerp` -180.0 -270.0 _swing) (`self.Return Value Y (Pitch)`) (`self.Return Value Z (Yaw)`)) false false)
      (`ActorComponent.K2_DestroyComponent` (`self.StaticMesh2`)))
    (:`Finished`
      (`GameplayStatics.PlaySound2D` "/Game/ElementalEchoes/Blueprints/Audio/Cues/pressure_plate_locked_Cue.pressure_plate_locked_Cue" 1.0 1.0 0.0 null null))))

(event `SwingPlatformUnactive`
  ; Animation for Platform Swing
  (`GameplayStatics.PlaySound2D` "/Game/ElementalEchoes/Blueprints/Audio/Cues/swing_platform_Cue.swing_platform_Cue" 1.0 1.0 0.0 null null)
  (goto _label :!via `Reverse`))

(fn `CheckToSeeHowManyPressurePlatesAreActive`
  (`self.IncreasePressurePlateActive`))

(fn `DecresePressurePlatesActive`
  (`/Engine/EditorBlueprintResources/StandardMacros.DecrementFloat` (`self.AmountofActiveObjects`)))

(fn `IncreasePressurePlateActive`
  (`/Engine/EditorBlueprintResources/StandardMacros.IncrementFloat` (`self.AmountofActiveObjects`)))

(fn `UserConstructionScript`)