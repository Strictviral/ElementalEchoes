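; Level actor for blocking roots that dissolve away on Interact, either permanently or with timed regrowth.
; Timelines drive the "Animation" material parameter and a matching Niagara float, with guard flags blocking re-triggering.
; The permanent path plays a burn sound, dissolves all static meshes, then destroys the actor.
; The regenerating path disables collision, waits, then restores it and reverses the dissolve, but never clears IsRegenerating, so later interactions are ignored.
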(event `self.ReceiveBeginPlay`)

(event `/Game/ElementalEchoes/Blueprints/Interface/BPI_Interact.Interact`
  (params (CharacterName :type String))
  ; Interact Interface To Handle Root Destruction
  (if (`self.bIsAbleToRegenerate`)
    (`self.StartDisintigrationWithRegeneration`)
    (else
      (`self.StartDisintigration`))))

(event `StartDisintigration`
  ; Disintegrate
  (if (not (or (`self.bIsDisintigrating`) (`self.bIsRegenerating`)))
    (set `self.bIsDisintigrating` true)
    (`GameplayStatics.PlaySound2D` "/Game/ElementalEchoes/Blueprints/Audio/Cues/burn_vine_Cue.burn_vine_Cue" 1.0 1.0 0.0 null null)
    (bind (_direction _dissolve) (`Timeline|Disintegration` :!via `PlayFromStart`)
      (:`Update`
        (for _array_element (`self.K2_GetComponentsByClass` "/Script/Engine.StaticMeshComponent")
          (`/Engine/EditorBlueprintResources/StandardMacros.IsValid` _array_element
            (:`Is Valid`
              (`MeshComponent.SetScalarParameterValueOnMaterials` _array_element "Animation" _dissolve)
              (`NiagaraComponent.SetNiagaraVariableFloat` (`self.Niagara`) "User_Animation" _dissolve)))))
      (:`Finished`
        (for _array_element_2 (`self.K2_GetComponentsByClass` "/Script/Engine.StaticMeshComponent")
          (`/Engine/EditorBlueprintResources/StandardMacros.IsValid` _array_element_2
            (:`Is Valid`
              (`PrimitiveComponent.SetCollisionEnabled` (`self.StaticMesh`) "NoCollision")
              (`PrimitiveComponent.SetCollisionEnabled` _array_element_2 "NoCollision")
              (`self.K2_DestroyActor`))))))))

(event `StartDisintigrationWithRegeneration`
  ; Disintegrate And Regenrate
  (if (not (or (`self.bIsDisintigrating`) (`self.bIsRegenerating`)))
    (set `self.bIsDisintigrating` true)
    (bind (_direction _dissolve) (`Timeline|DisintegrationR` :!via `PlayFromStart`)
      (:`Update`
        (`MeshComponent.SetScalarParameterValueOnMaterials` (`self.StaticMesh`) "Animation" _dissolve)
        (`NiagaraComponent.SetNiagaraVariableFloat` (`self.Niagara`) "User_Animation" _dissolve))
      (:`Finished`
        (set `self.bIsDisintigrating` false)
        (`PrimitiveComponent.SetCollisionEnabled` (`self.StaticMesh`) "NoCollision")
        (`KismetSystemLibrary.Delay` (`self.TimeUntilRegeneration`))
        (set `self.bIsRegenerating` true)
        (`PrimitiveComponent.SetCollisionEnabled` (`self.StaticMesh`) "QueryAndPhysics")
        (bind (_direction_2 _dissolve_2) (`Timeline|Regenerate` :!via `ReverseFromEnd`)
          (:`Update`
            (`MeshComponent.SetScalarParameterValueOnMaterials` (`self.StaticMesh`) "Animation" _dissolve_2)
            (`NiagaraComponent.SetNiagaraVariableFloat` (`self.Niagara`) "User_Animation" _dissolve_2)))))))

(fn `UserConstructionScript`)