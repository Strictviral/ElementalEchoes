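; BP_MovableSphere is a stone sphere level actor that the Earth character can push and pull.
; It caches the Earth character shortly after BeginPlay, and Interact toggles that character's attach or detach to the sphere.
; While pushed, Tick spins SpinMesh from the push input to show rolling.
; A separate Speed/Direction graph eases StoneMesh along its forward vector with VInterpTo.
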(event `self.ReceiveTick`
  (params (DeltaSeconds :type "Float (single-precision)"))
  (if (`self.bIsBeingPushed`)
    (`SceneComponent.K2_AddLocalRotation` (`self.SpinMesh`) (`KismetMathLibrary.MakeRotator` 0.0 (* (`self.CurrentPushInput`) (`self.RotationSpeed`) (`GameplayStatics.GetWorldDeltaSeconds`))) false false)))

(event `self.ReceiveBeginPlay`
  (`KismetSystemLibrary.Delay` 0.5)
  (bind _returnvalue (`GameplayStatics.GetActorOfClass` "/Game/ElementalEchoes/Blueprints/Character/BP_EarthCharacter.BP_EarthCharacter_C"))
  (set `self.EarthCharacterRef` _returnvalue))

(event `self.Interact`
  ; Interact Event For Pushing and Pulling
  (if (not (`/Game/ElementalEchoes/Blueprints/Character/BP_EarthCharacter.bIsInteracting` (`self.EarthCharacterRef`)))
    (`/Game/ElementalEchoes/Blueprints/Character/BP_EarthCharacter.CheckandAttachMovingObjectSphere` (`self.EarthCharacterRef`))
    (else
      (`/Game/ElementalEchoes/Blueprints/Character/BP_EarthCharacter.DetachFromMovingObjectSphere` (`self.EarthCharacterRef`)))))

(fn `UserConstructionScript`)