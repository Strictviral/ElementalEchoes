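; BP_FireballLauncher is a level hazard that fires fireballs while the player is within range.
; Its Sphere overlap starts a looping timer at FireRate when a Player-tagged actor enters, and clears it by stored handle when one leaves.
; Each tick of the timer spawns a BP_FireballEnv at the CannonHeadPoint location and rotation and plays an attenuated launch sound at the launcher.
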(event `self.ReceiveBeginPlay`)

(event `self.Sphere.OnComponentBeginOverlap`
  (params (OverlappedComponent :type "PrimitiveComponent Object Reference") (OtherActor :type "Actor Object Reference") (OtherComp :type "PrimitiveComponent Object Reference") (OtherBodyIndex :type Integer) (bFromSweep :type Boolean) (SweepResult :type "HitResult Structure (by ref)"))
  ; Activate Fireball Launcher
  (if (`self.ActorHasTag` OtherActor "Player")
    (bind _returnvalue (`KismetSystemLibrary.K2_SetTimerDelegate` (delegate `ShootFireball`) (`self.FireRate`) true))
    (set `self.Funtionhandlers` _returnvalue)))

(event `ShootFireball`
  (bind _cannonheadpoint (`self.CannonHeadPoint`))
  ; Activate Fireball Launcher
  (`|SpawnActorFromClass` "/Game/ElementalEchoes/Blueprints/Projectiles/BP_FireballEnv.BP_FireballEnv_C" (`KismetMathLibrary.MakeTransform` (`SceneComponent.K2_GetComponentLocation` _cannonheadpoint) (`SceneComponent.K2_GetComponentRotation` _cannonheadpoint)) "Undefined" "MultiplyWithRoot" null null)
  (`GameplayStatics.PlaySoundAtLocation` "/Game/ElementalEchoes/Blueprints/Audio/Cues/fireball_launcher_Cue.fireball_launcher_Cue" (`self.K2_GetActorLocation`) (struct) 1.0 1.0 0.0 "/Game/ElementalEchoes/Blueprints/Audio/FireBallLauncherSoundAttenuation.FireBallLauncherSoundAttenuation" null null null))

(event `self.Sphere.OnComponentEndOverlap`
  (params (OverlappedComponent :type "PrimitiveComponent Object Reference") (OtherActor :type "Actor Object Reference") (OtherComp :type "PrimitiveComponent Object Reference") (OtherBodyIndex :type Integer))
  ; Deactivate Fireball Launcher
  (if (`self.ActorHasTag` OtherActor "Player")
    (`KismetSystemLibrary.K2_ClearAndInvalidateTimerHandle` (`self.Funtionhandlers`))))

(fn `UserConstructionScript`)