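; A level checkpoint actor that records its own location as the player's most recent checkpoint.
; On BeginPlay it caches the player character and the elemental game instance.
; When that player overlaps the checkpoint box while it is active, it passes its location to the game instance and deactivates itself, so it triggers only once.
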(event `self.ReceiveBeginPlay`
  (bind _asbp_base_character (cast `/Game/ElementalEchoes/Blueprints/Character/BP_BaseCharacter` (`GameplayStatics.GetPlayerCharacter` 0)))
  (set `self.Player` _asbp_base_character)
  (bind _asbp_elemental_game_instance (cast `/Game/ElementalEchoes/Blueprints/GameInstance/BP_ElementalGameInstance` (`GameplayStatics.GetGameInstance`)))
  (set `self.ElementalGameInstance` _asbp_elemental_game_instance))

(event `self.CheckPointBox.OnComponentBeginOverlap`
  (params (OverlappedComponent :type "PrimitiveComponent Object Reference") (OtherActor :type "Actor Object Reference") (OtherComp :type "PrimitiveComponent Object Reference") (OtherBodyIndex :type Integer) (bFromSweep :type Boolean) (SweepResult :type "HitResult Structure (by ref)"))
  (if (and (== OtherActor (`self.Player`)) (`self.bIsActive`))
    (bind _actorlocation (`self.GetActorLocation`))
    (`/Game/ElementalEchoes/Blueprints/GameInstance/BP_ElementalGameInstance.SetRecentCheckpoint` (`self.ElementalGameInstance`) _actorlocation)
    (set `self.bIsActive` false)))

(fn `GetActorLocation`
  (returns (ActorLocation :type "Vector Structure"))
  (return (`self.K2_GetActorLocation`)))

(fn `UserConstructionScript`)