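; BP_SwingPlatform_V is a level actor platform that swings open when all of its linked trigger objects, such as pressure plates, are active.
; On BeginPlay it counts the OpenObjects and binds to their active and inactive events, and also binds to Lever activation.
; Each change updates an active count and compares it to the total.
; A timeline rolls the mesh through a quarter turn, reversing when the count falls short.
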(event `self.ReceiveBeginPlay`
  ; Initialized and find all actors
  (for _array_element (`self.OpenObjects`)
    (`/Engine/EditorBlueprintResources/StandardMacros.IncrementFloat` (`self.AmountofObjectsFound`)
      (:`  `
        (add `/Game/ElementalEchoes/Blueprints/PuzzleActors/BP_OpenObjects.ObjectActive` _array_element (delegate `SwingPlatformOpen`))
        (add `/Game/ElementalEchoes/Blueprints/PuzzleActors/BP_OpenObjects.ObjectsInactive` _array_element (delegate `SwingPlatformClosed`)))))
  (for _array_element_2 (`self.Lever`)
    (add `/Game/ElementalEchoes/Blueprints/PuzzleActors/BP_Lever.LeverActivate` _array_element_2 (`|CreateDelegate` :!event `SwingPlatformActive`))))

(event `SwingPlatformOpen`
  ; Initialized and find all actors
  (`self.IncreasePressurePlateActive`)
  (`self.CheckPlatforms`))

(event `SwingPlatformClosed`
  ; Initialized and find all actors
  (`self.DecresePressurePlatesActive`)
  (`self.CheckPlatforms`))

(event `CheckPlatforms`
  ; Check to see if Pressur plates are active
  (if (>= (`self.AmountofActiveObjects`) (`self.AmountofObjectsFound`))
    (`self.SwingPlatformActive`)
    (else
      (`self.SwingPlatformUnactive`))))

(event `SwingPlatformActive`
  ; Animation for Platform Swing
  (bind (_direction _swing) (`Timeline|Timeline` :!label _label)
    (:`Update`
      (`SceneComponent.K2_SetRelativeRotation` (`self.StaticMesh`) (`KismetMathLibrary.MakeRotator` (`KismetMathLibrary.Lerp` -90.0 0.0 _swing)) false false))))

(event `SwingPlatformUnactive`
  ; Animation for Platform Swing
  (goto _label :!via `Reverse`))

(fn `CheckToSeeHowManyPressurePlatesAreActive`
  (`self.IncreasePressurePlateActive`))

(fn `DecresePressurePlatesActive`
  (`/Engine/EditorBlueprintResources/StandardMacros.DecrementFloat` (`self.AmountofActiveObjects`)))

(fn `IncreasePressurePlateActive`
  (`/Engine/EditorBlueprintResources/StandardMacros.IncrementFloat` (`self.AmountofActiveObjects`)))

(fn `UserConstructionScript`)